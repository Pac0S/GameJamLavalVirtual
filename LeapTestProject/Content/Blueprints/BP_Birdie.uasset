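; BP_Birdie is a physics-driven birdie (apparently a shuttlecock) that can be teleported through portals and projects a floor target beneath itself.
; PortalTo moves BirdieCap to the given location with clamped height, applies the rotation, and sets CanTeleport.
; It redirects velocity by swapping X and Z with a sign flip, clamped to launch upward toward negative X, and prints debug values.
; Tick keeps FloorTarget under the cap at fixed height.
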(event `PortalTo`
  (params (Location :type "Vector Structure") (Rotation :type "Rotator Structure"))
  (bind _birdie_cap (`self.Birdie_Cap`))
  (bind _returnvalue (`SceneComponent.GetComponentVelocity` _birdie_cap))
  (bind _returnvalue_2 (`KismetMathLibrary.MakeVector` (.x Location) (.y Location) (`KismetMathLibrary.FClamp` (.z Location) 300.0 500.0)))
  (bind _returnvalue_3 (`KismetMathLibrary.MakeVector` (`KismetMathLibrary.FClamp` (.x (`KismetMathLibrary.MakeVector` (.z _returnvalue) 0.0 (- 0.0 (.x _returnvalue)))) -1000.0 -300.0) 0.0 (`KismetMathLibrary.FClamp` (.z (`KismetMathLibrary.MakeVector` (.z _returnvalue) 0.0 (- 0.0 (.x _returnvalue)))) 300.0 1000.0)))
  ;[1 1 1] Set new position, rotation and speed for birdie
  (`PrimitiveComponent.GetPhysicsLinearVelocity` _birdie_cap "None")
  (`KismetSystemLibrary.PrintString` (`KismetStringLibrary.Concat_StrStr` "INITIAL SPEED : " (`KismetStringLibrary.Conv_VectorToString` _returnvalue)) true true (struct :`G` 0.66 :`B` 1.0 :`A` 1.0) 30.0)
  (`KismetSystemLibrary.PrintString` (`KismetStringLibrary.Concat_StrStr` "SPAWN POSITION" (`KismetStringLibrary.Conv_VectorToString` _returnvalue_2)) true true (struct :`G` 0.66 :`B` 1.0 :`A` 1.0) 30.0)
  (`SceneComponent.K2_SetWorldLocation` _birdie_cap _returnvalue_2 false true)
  (`SceneComponent.K2_SetWorldRotation` _birdie_cap Rotation false true)
  (`PrimitiveComponent.SetAllPhysicsLinearVelocity` (`self.Birdie_Cap`) _returnvalue_3 false)
  (`KismetSystemLibrary.PrintString` (`KismetStringLibrary.Concat_StrStr` "SPEED : " (`KismetStringLibrary.Conv_VectorToString` _returnvalue_3)) true true (struct :`G` 0.66 :`B` 1.0 :`A` 1.0) 30.0)
  (`KismetSystemLibrary.PrintString` "" true true (struct :`G` 0.66 :`B` 1.0 :`A` 1.0) 30.0)
  (set `self.CanTeleport` true))

(event `self.ReceiveTick`
  (params (DeltaSeconds :type "Float (single-precision)"))
  (`SceneComponent.K2_SetWorldLocation` (`self.FloorTarget`) (`KismetMathLibrary.MakeVector` (.x (`SceneComponent.K2_GetComponentLocation` (`self.Birdie_Cap`))) (.y (`SceneComponent.K2_GetComponentLocation` (`self.Birdie_Cap`))) 30.0) false false))

(fn `UserConstructionScript`)