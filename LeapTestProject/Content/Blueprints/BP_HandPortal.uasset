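; BP_HandPortal is a portal actor that teleports the birdie to the net portal when the birdie hits its plane.
; The hit event finds the first BP_Birdie and BP_NetPortal, and uses the birdie's CanTeleport flag, cleared on use, to gate the jump.
; The exit takes the net portal's X, keeps the birdie's Y, converts its X into an inverted height and adds a quarter-turn of pitch.
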(event `self.PortalPlane.OnComponentHit`
  (params (HitComponent :type "PrimitiveComponent Object Reference") (OtherActor :type "Actor Object Reference") (OtherComp :type "PrimitiveComponent Object Reference") (NormalImpulse :type "Vector Structure") (Hit :type "HitResult Structure (by ref)"))
  (bind _volant (`self.Volant`))
  (bind _birdie_cap (`/Game/Blueprints/BP_Birdie.Birdie_Cap` (`self.Volant`)))
  ;[1 1 1] Get collision between birdie and portal
  (bind _outactors (`GameplayStatics.GetAllActorsOfClass` "/Game/Blueprints/BP_Birdie.BP_Birdie_C"))
  (bind _output (`|GetArrayItem` _outactors))
  (if (== _output OtherActor)
    (set `self.Volant` _output)
    ;[1 1 1] Make teleport location for birdie
    (bind _outactors_2 (`GameplayStatics.GetAllActorsOfClass` "/Game/Blueprints/BP_NetPortal.BP_NetPortal_C"))
    ;[1 1 1] Teleport birdie
    (if (`/Game/Blueprints/BP_Birdie.CanTeleport` _volant)
      (set `/Game/Blueprints/BP_Birdie.CanTeleport` false _volant)
      (`/Game/Blueprints/BP_Birdie.PortalTo` _volant (`KismetMathLibrary.MakeVector` (.x (`SceneComponent.K2_GetComponentLocation` (`/Game/Blueprints/BP_NetPortal.PortalPlane` (`|GetArrayItem` _outactors_2)))) (.y (`SceneComponent.K2_GetComponentLocation` _birdie_cap)) (- 300.0 (- (.x (`SceneComponent.K2_GetComponentLocation` _birdie_cap)) 130.0))) (`KismetMathLibrary.MakeRotator` (.roll (`SceneComponent.K2_GetComponentRotation` _birdie_cap)) (+ (.pitch (`SceneComponent.K2_GetComponentRotation` _birdie_cap)) 90.0) (.yaw (`SceneComponent.K2_GetComponentRotation` _birdie_cap)))))))

(fn `UserConstructionScript`)